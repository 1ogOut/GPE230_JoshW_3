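; MazeCharacterBP is the maze player character Blueprint, providing an area stun ability against enemies.
; The Stun input, gated by a cooldown that Tick counts down, plays a particle effect and sphere-traces around the character by object type.
; Hit NPCEnemyButWithABP actors are told to become stunned; the loop stops at the first failed cast.
; A debug M key applies damage to the character itself.
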(event `InputAction|Stun`
  (params (Key :type "Key Structure"))
  (bind _returnvalue (`self.K2_GetActorLocation`))
  ; stun enemy
  (:`Pressed`
    (if (<= (`self.StunCooldown`) 0.0)
      (set `self.StunCooldown` (`self.TimeBetweenStuns`))
      (`self.ActivateStunParticleSystem`)
      (bind _outhits (`KismetSystemLibrary.SphereTraceMultiForObjects` _returnvalue _returnvalue (`self.StunTraceRadius`) (`self.StunTraceTypes`)))
      (for _array_element _outhits
        (bind _asnpcenemy_but_with_abp (cast `/Game/EnemyAI/NPCEnemyButWithABP` (`.HitActor` (`GameplayStatics.BreakHitResult` _array_element))))
        (`/Game/EnemyAI/NPCEnemyButWithABP.Stunned` _asnpcenemy_but_with_abp)))))

(event `self.ReceiveTick`
  (params (DeltaSeconds :type "Float (single-precision)"))
  ; if stun cooldown is over 0 subtract from it every second
  (if (> (`self.StunCooldown`) 0.0)
    (set `self.StunCooldown` (- (`self.StunCooldown`) DeltaSeconds))))

(event `Key|M`
  (params (Key :type "Key Structure"))
  ; damage player (to test)
  (:`Pressed`
    (`GameplayStatics.ApplyDamage` self 1.0)))

(fn `UserConstructionScript`)