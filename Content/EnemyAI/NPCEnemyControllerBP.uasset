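; AI controller for enemy NPCs that runs the NPCEnemyBT behavior tree and feeds its blackboard.
; BeginPlay stores the location of a GuardPoint actor as GuardPosition.
; Perception updates set TargetActor to the reported actor, with no filter for player or sensing success.
; While a target is valid, Tick writes its distance from the controlled pawn to DistanceToPlayer and prints it on screen for debugging.
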(event `self.ReceiveBeginPlay`
  ; when the game starts, have the AI move to the target(GuardPoint Actor) if the target doesn't exist(or is out of reach) it will run randomly
  (bind _returnvalue (`GameplayStatics.GetActorOfClass` "/Game/EnemyAI/GuardPoint.GuardPoint_C"))
  (`self.RunBehaviorTree` "/Game/EnemyAI/NPCEnemyBT.NPCEnemyBT")
  (`BlackboardComponent.SetValueAsVector` (`AIBlueprintHelperLibrary.GetBlackboard` null) "GuardPosition" (`self.K2_GetActorLocation` _returnvalue)))

(event `self.AIPerception.OnTargetPerceptionUpdated`
  (params (Actor :type "Actor Object Reference") (Stimulus :type "AIStimulus Structure"))
  ; run to player if it sees them
  (`BlackboardComponent.SetValueAsObject` (`AIBlueprintHelperLibrary.GetBlackboard` null) "TargetActor" Actor))

(event `self.ReceiveTick`
  (params (DeltaSeconds :type "Float (single-precision)"))
  (bind _returnvalue (`BlackboardComponent.GetValueAsObject` (`AIBlueprintHelperLibrary.GetBlackboard` null) "TargetActor"))
  (if (`KismetSystemLibrary.IsValid` _returnvalue)
    (bind _asactor (cast `Actor` _returnvalue))
    (bind _returnvalue_2 (`self.GetDistanceTo` _asactor (`self.K2_GetPawn`)))
    (`BlackboardComponent.SetValueAsFloat` (`AIBlueprintHelperLibrary.GetBlackboard` null) "DistanceToPlayer" _returnvalue_2)
    (`KismetSystemLibrary.PrintString` (`KismetStringLibrary.Conv_DoubleToString` _returnvalue_2) true false (struct :`G` 0.66 :`B` 1.0 :`A` 1.0) 0.025)))

(fn `UserConstructionScript`)